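; Placement preview dummy for turrets that shows whether its current spot is clear.
; Actor overlap begin and end swap the static mesh material between bad and good placement, without counting simultaneous overlaps.
; Active and LockXY start false on BeginPlay, and this file never changes them afterwards.
; Tick re-enables physics simulation on the mesh every frame while Active is true and LockXY is false.
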(event `self.ReceiveTick`
  (params (DeltaSeconds :type "Float (single-precision)"))
  (if (stale `self.ReceiveBeginPlay` _output_get)
    (if (not (stale `self.ReceiveBeginPlay` _output_get_2))
      (`PrimitiveComponent.SetSimulatePhysics` (`self.StaticMesh`) true))))

(event `self.ReceiveBeginPlay`
  (bind _output_get (set `self.active` false))
  (bind _output_get_2 (set `self.lock x y` false)))

(event `self.ReceiveActorBeginOverlap`
  (params (OtherActor :type "Actor Object Reference"))
  (`PrimitiveComponent.SetMaterial` (`self.StaticMesh`) 0 "/Game/Materials/turretPlaceBad.turretPlaceBad"))

(event `self.ReceiveActorEndOverlap`
  (params (OtherActor :type "Actor Object Reference"))
  (`PrimitiveComponent.SetMaterial` (`self.StaticMesh`) 0 "/Game/Materials/turretPlaceGood.turretPlaceGood"))

(fn `UserConstructionScript`)