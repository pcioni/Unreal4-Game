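; Behavior tree task for basic AI that makes the AI follow the player when within a fixed range.
; On execute, it measures the distance between the owner actor and the first player pawn.
; If close enough, it writes the player's current location to the Destination blackboard key and succeeds; otherwise it fails.
; It only sets the destination and does no movement itself.
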(event `self.ReceiveExecute`
  (params (OwnerActor :type "Actor Object Reference"))
  ;[1 1 1] Determines Distance to Player
  (if (<= (`KismetMathLibrary.VSize` (- (`Actor.K2_GetActorLocation` OwnerActor) (`Actor.K2_GetActorLocation` (`GameplayStatics.GetPlayerPawn` 0)))) 2000.0)
    ;[1 1 1] If close, follow the player.
    (`BTFunctionLibrary.SetBlackboardValueAsVector` (`self.Destination`) (`Actor.K2_GetActorLocation` (`GameplayStatics.GetPlayerPawn` 0)))
    (`self.FinishExecute` true)
    (else
      ;[1 1 1] If far away, break.
      (`self.FinishExecute` false))))