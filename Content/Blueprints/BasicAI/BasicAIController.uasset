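; BasicAIController is an AI controller that runs BasicBehaviorTree on BeginPlay and attempts a random loot drop when the controller itself is destroyed.
; DropGoodies makes up to three chained random rolls, drawing a fresh number at each check, so the three goodies have unequal odds and often none is chosen.
; The three SpawnGoody functions it calls are empty stubs, so nothing actually spawns.
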(event `self.ReceiveBeginPlay`
  (`self.RunBehaviorTree` "/Game/Blueprints/BasicAI/BasicBehaviorTree.BasicBehaviorTree"))

(event `self.ReceiveTick`
  (params (DeltaSeconds :type "Float (single-precision)")))

(event `self.ReceiveDestroyed`
  (`self.DropGoodies`))

(fn `DropGoodies`
  (bind _returnvalue (`KismetMathLibrary.RandomIntegerInRange` 0 5))
  (if (== _returnvalue 0)
    (`self.SpawnGoody1`)
    (elif (== _returnvalue 1)
      (`self.SpawnGoody2`)
      (elif (== _returnvalue 2)
        (`self.SpawnGoody3`)))))

(fn `SpawnGoody1`)

(fn `SpawnGoody2`)

(fn `SpawnGoody3`)

(fn `UserConstructionScript`)