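; Behavior tree task for basic AI that moves the owning actor one step along a direction read from the blackboard.
; On execute it normalizes the Direction vector, scales it by frame delta time and a hardcoded speed, and adds it to the actor's location.
; The transform is set as a teleport without sweep, and the task immediately finishes successfully.
; The Speed variable is unused.
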(event `self.ReceiveExecute`
  (params (OwnerActor :type "Actor Object Reference"))
  (`Actor.K2_SetActorTransform` OwnerActor (`KismetMathLibrary.MakeTransform` (+ (* (`KismetMathLibrary.Normal` (`BTFunctionLibrary.GetBlackboardValueAsVector` (`self.Direction`))) (* (`GameplayStatics.GetWorldDeltaSeconds`) 500.0)) (.location (`Actor.GetTransform` OwnerActor))) (.rotation (`Actor.GetTransform` OwnerActor)) (.scale (`Actor.GetTransform` OwnerActor))) false true)
  (`self.FinishExecute` true))