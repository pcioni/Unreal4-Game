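; Ranged AI character that attacks with a Cannon component and shows its health on a floating widget bar.
; Each tick it calls Fire on the cannon, copies the Damageable component's health fraction into the bar, and yaws the bar toward player 0 using a flattened direction vector.
; When destroyed, it calls SpawnGoodies.
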(event `self.ReceiveBeginPlay`)

(event `self.ReceiveActorBeginOverlap`
  (params (OtherActor :type "Actor Object Reference")))

(event `self.ReceiveTick`
  (params (DeltaSeconds :type "Float (single-precision)"))
  (`/Game/Cannon.Fire` (`self.Cannon`))
  ;[1 1 1] update health bar
  (bind _asaihealth_bar (cast `/Game/AIhealthBar` (`WidgetComponent.GetUserWidgetObject` (`self.health bar`))))
  (bind _health_fraction (`/Game/Damageable.GetHealthFraction` (`self.Damageable`)))
  (`ProgressBar.SetPercent` (`/Game/AIhealthBar.ProgressBar_29` _asaihealth_bar) _health_fraction)
  (`SceneComponent.K2_SetWorldRotation` (`self.health bar`) (`KismetMathLibrary.Conv_VectorToRotator` (`KismetMathLibrary.GreaterGreater_VectorRotator` (`KismetMathLibrary.Normal` (* (- (`self.K2_GetActorLocation` (`GameplayStatics.GetPlayerPawn` 0)) (`self.K2_GetActorLocation`)) (1.0 1.0 0.0))))) false false))

(event `self.ReceiveDestroyed`
  (`self.SpawnGoodies`))

(fn `UserConstructionScript`
  (`parent.UserConstructionScript`))