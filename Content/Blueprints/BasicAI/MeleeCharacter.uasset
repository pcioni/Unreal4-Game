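; Melee AI character that periodically swings a Cube weapon and damages what it touches.
; Tick runs the parent logic, then MoveWeapon, which toggles swing state on alternating long and short real-time delays, applying a one-off lerped local rotation each time.
; Cube overlaps call HitPerson, which damages the other actor's first Damageable component unless its Side is Enemy, and plays a punch sound.
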(event OnComponentHit(Cube)
  (params (OtherActor :type Actor%20Object%20Reference) (OtherComp :type Primitive%20Component%20Object%20Reference) (NormalImpulse :type Vector :default "0, 0, 0") (Hit :type Hit%20Result%20Structure%20%28by%20ref%29)))

(event OnComponentBeginOverlap(Cube)
  (params (OtherActor :type Actor%20Object%20Reference) (OtherComp :type Primitive%20Component%20Object%20Reference) (OtherBodyIndex :type Integer) (bFromSweep :type Boolean) (SweepResult :type Hit%20Result%20Structure%20%28by%20ref%29))
  (CallFunction|HitPerson OtherActor))

(event EventBeginPlay)

(event EventActorBeginOverlap
  (params (OtherActor :type Actor%20Object%20Reference)))

(event EventTick
  (params (DeltaSeconds :type Float%20%28single-precision%29))
  (|CallParentFunction 0.0)
  (CallFunction|MoveWeapon DeltaSeconds))

(fn ConstructionScript
  (|CallParentFunction))

(fn HitPerson
  (params (OtherGuy :type Actor%20Object%20Reference))
  (bind _returnvalue (Actor|GetComponentsByClass OtherGuy "/Game/Damageable.Damageable_C"))
  (bind _item (Utilities|Array|Get(acopy) _returnvalue))
  (if (not (Utilities|Enum|Equal(Enum) (Variables|/Game/Damageable.Damageable_C|GetSide _item) "Enemy"))
    (Default|TakeDamage _item 5)
    (Audio|SpawnSoundatLocation "/Game/Sounds/batman_punch.batman_punch" (Transformation|GetSocketLocation (Variables|Default|GetCube) "None"))))

(fn MoveWeapon
  (params (Delta :type Float%20%28single-precision%29))
  (bind _returnvalue (Utilities|Time|GetRealTimeSeconds))
  (bind _cube (Variables|Default|GetCube))
  (if (<= (Variables|Default|GetnextSwing) _returnvalue)
    (if (Variables|Default|GetswingingUp)
      (Variables|Default|SetnextSwing (+ _returnvalue 1.0))
      (else
        (Variables|Default|SetnextSwing (+ _returnvalue 0.1))))
    (Components|StaticMesh|SetStaticMesh _cube (Variables|/Script/Engine.StaticMeshComponent|GetStaticMesh (Variables|Default|GetCube)))
    (if (Variables|Default|GetswingingUp)
      (Variables|Default|SetswingingUp false)
      (Transformation|AddLocalRotation _cube (Math|Rotator|Lerp(Rotator) "90.000000,0.000000,0.000000" "0.000000,0.000000, 0" (/ Delta 1.0)) false false)
      (else
        (Variables|Default|SetswingingUp true)
        (Transformation|AddLocalRotation _cube (Math|Rotator|Lerp(Rotator) "0.000000,0.000000,0.000000" "90.000000,0.000000, 0" (/ Delta 1.0)) false false)))))