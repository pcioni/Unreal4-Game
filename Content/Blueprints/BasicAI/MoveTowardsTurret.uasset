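; Behavior tree task that sends an AI toward the nearest TestTurret within a fixed range.
; FindClosest linearly scans all TestTurret actors for the shortest distance, storing the turret and its location.
; In range, it writes the Destination blackboard key and issues MoveToActor, finishing without waiting for arrival.
; FindClosest itself calls FinishExecute(true), so success is reported before the range check can report failure.
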(event `self.ReceiveExecute`
  (params (OwnerActor :type "Actor Object Reference"))
  (`self.FindClosest` OwnerActor)
  (if (< (`self.ClosestDistance`) 2500.0)
    (`BTFunctionLibrary.SetBlackboardValueAsVector` (`self.Destination`) (`self.ClosestVector`))
    (bind _returnvalue (`AIBlueprintHelperLibrary.GetAIController` OwnerActor))
    (`AIController.MoveToActor` _returnvalue (`self.targetTurret`) 200.0 true true true null true)
    (`self.FinishExecute` true)
    (else
      (`self.FinishExecute` false))))

(fn `FindClosest`
  (params (Selff :type "Actor Object Reference"))
  (set `self.ClosestDistance` 9999999999.0)
  (bind _outactors (`GameplayStatics.GetAllActorsOfClass` "/Game/Turrets/testTurret.testTurret_C"))
  (for _array_element _outactors
    (bind _returnvalue (`KismetMathLibrary.VSize` (- (`Actor.K2_GetActorLocation` Selff) (`Actor.K2_GetActorLocation` _array_element))))
    (if (< _returnvalue (`self.ClosestDistance`))
      (set `self.ClosestDistance` _returnvalue)
      (set `self.ClosestVector` (`Actor.K2_GetActorLocation` _array_element))
      (set `self.targetTurret` _array_element)))
  (`self.FinishExecute` true))