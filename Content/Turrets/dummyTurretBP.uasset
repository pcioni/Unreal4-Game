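; Dummy turret that acts as a placement preview, tracking whether its spot is valid through a Placeable flag.
; On overlap begin it scans the other actor's overlapping components, marking the spot bad until it finds one tagged "ignore".
; It swaps good and bad placement materials to match, and any overlap end resets it to placeable.
; While Active is set, Tick enables physics simulation on the mesh.
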(event `self.ReceiveTick`
  (params (DeltaSeconds :type "Float (single-precision)"))
  (if (stale `self.ReceiveBeginPlay` _output_get)
    (`PrimitiveComponent.SetSimulatePhysics` (`self.StaticMesh`) true)))

(event `self.ReceiveBeginPlay`
  (set `self.placeable` true)
  (bind _output_get (set `self.active` false)))

(event `self.ReceiveActorBeginOverlap`
  (params (OtherActor :type "Actor Object Reference"))
  (bind _staticmesh (`self.StaticMesh`))
  (for _array_element (`self.GetOverlappingComponents` OtherActor)
    (if (`ActorComponent.ComponentHasTag` _array_element "ignore")
      (set `self.placeable` true)
      (`PrimitiveComponent.SetMaterial` _staticmesh 0 "/Game/Materials/turretPlaceGood.turretPlaceGood")
      (break)
      (else
        (set `self.placeable` false)
        (`PrimitiveComponent.SetMaterial` _staticmesh 0 "/Game/Materials/turretPlaceBad.turretPlaceBad")))))

(event `self.ReceiveActorEndOverlap`
  (params (OtherActor :type "Actor Object Reference"))
  (set `self.placeable` true)
  (`PrimitiveComponent.SetMaterial` (`self.StaticMesh`) 0 "/Game/Materials/turretPlaceGood.turretPlaceGood"))

(fn `UserConstructionScript`)